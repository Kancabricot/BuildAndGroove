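; Grid actor that builds a board of BP_Case tiles plus a separate player row, and spawns characters on them.
; The construction script creates tiles as child actors, records their indices and flags back rows as spawnable.
; BeginPlay fills every player-row tile with a BP_PlayerOnStage.
; SpawnEnemy places an enemy on a random unoccupied grid tile, checking only occupancy, not the spawnable flag.
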(event EventBeginPlay
  (CallFunction|SpawnPlayer))

(fn ConstructionScript
  (CallFunction|CreateGrid))

(fn CreateGrid
  (bind _returnvalue (Transformation|GetActorLocation))
  (bind _returnvalue_2 (Transformation|GetActorLocation))
  (bind (_x _y) (Math|Vector|BreakVector _returnvalue))
  (bind (_x_2 _y_2) (Math|Vector|BreakVector _returnvalue_2))
  (Utilities|Array|Clear (Variables|Default|GetStruc_Grid))
  (Utilities|Array|Clear (Variables|Default|GetStruc_PlayerGrid))
  (for _index (range 0 (- (Variables|Default|GetNombreCaseY) 1))
    (for _index_2 (range 0 (- (Variables|Default|GetNombreCaseX) 1))
      (bind _returnvalue_3 (AddComponent|AddChildActorComponent true (Math|Transform|MakeTransform (Math|Vector|MakeVector (+ (* _index 100) _x_2) (+ (* _index_2 100) _y_2) 0.0) "0, 0, 0" "1.000000,1.000000,1.000000")))
      (bind _asbp_case (Utilities|Casting|CastToBP_Case (Variables|/Script/Engine.ChildActorComponent|GetChildActor _returnvalue_3)))
      (Variables|/Game/01-Blueprints/03-Grid/BP_Case.BP_Case_C|SetIndexPos _asbp_case (Math|Vector2D|MakeVector2D (Math|Conversions|ToFloat(Integer) _index_2) (Math|Conversions|ToFloat(Integer) _index)))
      (Default|SetTextDebug _asbp_case)
      (Utilities|Array|Add (Variables|Default|GetStruc_Grid) (Utilities|Struct|MakeStruc_Grid _asbp_case (Math|Vector2D|MakeVector2D (Math|Conversions|ToFloat(Integer) _index_2) (Math|Conversions|ToFloat(Integer) _index)) (CallFunction|CheckifCanSpawn _index (Variables|Default|GetNombreCaseY))))))
  (for _index_3 (range 0 (- (Variables|Default|GetNombreCaseX) 1))
    (bind _returnvalue_4 (AddComponent|AddChildActorComponent true (Math|Transform|MakeTransform (Math|Vector|MakeVector (- _x 1.5e+02) (+ (* _index_3 100) _y) 0.0) "0, 0, 0" "1.000000,1.000000,1.000000")))
    (bind _asbp_case_2 (Utilities|Casting|CastToBP_Case (Variables|/Script/Engine.ChildActorComponent|GetChildActor _returnvalue_4)))
    (Utilities|Array|Add (Variables|Default|GetStruc_PlayerGrid) (Utilities|Struct|MakeStruc_Grid _asbp_case_2 (Math|Vector2D|MakeVector2D (Math|Conversions|ToFloat(Integer) _index_3) -1.0) false))))

(fn CheckifCanSpawn
  (params (IndexY :type Integer) (MaxIndex :type Integer))
  (return (> IndexY (- MaxIndex (- (Variables|Default|GetNombreCaseFondPourSpawn) 1)))))

(fn SpawnPlayer
  (for _array_element (Variables|Default|GetStruc_PlayerGrid)
    (bind _returnvalue (Game|SpawnActorfromClass "/Game/01-Blueprints/01-Game/BP_PlayerOnStage.BP_PlayerOnStage_C" (Transformation|GetWorldTransform (Variables|/Game/01-Blueprints/03-Grid/BP_Case.BP_Case_C|GetTopOfCase (.Case (Utilities|Struct|BreakStruc_Grid _array_element)))) "AlwaysSpawn" "MultiplyWithRoot" 0 (.Case (Utilities|Struct|BreakStruc_Grid _array_element)) 0))
    (Default|OnAttached (.Case (Utilities|Struct|BreakStruc_Grid _array_element)) _returnvalue)))

(fn SpawnEnemy
  (params (Class :type Actor%20Class%20Reference))
  (bind _temparrayofspawn (LocalVariables|GetTempArrayOfSpawn))
  (bind _asbp_parent_enemy (Utilities|Casting|CastToBP_ParentEnemyClass Class))
  (for _array_element (Variables|Default|GetStruc_Grid)
    (if (not (Variables|/Game/01-Blueprints/03-Grid/BP_Case.BP_Case_C|Getb_HaveSomethingOn (.case _array_element)))
      (Utilities|Array|Add (LocalVariables|GetTempArrayOfSpawn) (.case _array_element))))
  (if (Utilities|Array|IsEmpty _temparrayofspawn)
    (return)
    (else
      (bind _output_get (LocalVariables|SetCaseTemp (.OutItem (Utilities|Array|Random _temparrayofspawn))))
      (bind _returnvalue (Game|SpawnActorfromClass _asbp_parent_enemy (Transformation|GetWorldTransform (Variables|/Game/01-Blueprints/03-Grid/BP_Case.BP_Case_C|GetTopOfCase _output_get)) "AlwaysSpawn" "MultiplyWithRoot" 0 (LocalVariables|GetCaseTemp) 0))
      (Default|OnAttached (LocalVariables|GetCaseTemp) _returnvalue)
      (return))))