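; BP_Case is a grid tile that rises when hovered and can carry an attached actor.
; A timeline, played on hover and reversed on unhover, lerps the BPCase component's Z offset from its position cached at BeginPlay.
; OnAttached snaps the given actor to the TopOfCase component and flags the tile as occupied, while OnDetached clears the flag and detaches any valid actor.
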(event Custom|OnHover
  (bind _newtrack_0 (Timeline|Hover/Unhover Play)
    (:Update
      (Transformation|SetRelativeLocation (Variables|Default|GetBP_Case) (Math|Vector|MakeVector 0.0 0.0 (+ (.z (Variables|Default|GetInitialPosCase)) (Math|Float|Lerp 0.0 2e+01 _newtrack_0))) false false))))

(event Custom|OnUnhover
  (bind _newtrack_0 (Timeline|Hover/Unhover Reverse)
    (:Update
      (Transformation|SetRelativeLocation (Variables|Default|GetBP_Case) (Math|Vector|MakeVector 0.0 0.0 (+ (.z (Variables|Default|GetInitialPosCase)) (Math|Float|Lerp 0.0 2e+01 _newtrack_0))) false false))))

(event EventBeginPlay
  (Variables|Default|SetInitialPosCase (Variables|/Script/Engine.SceneComponent|GetRelativeLocation (Variables|Default|GetBP_Case))))

(fn ConstructionScript)

(fn OnAttached
  (params (Target :type Actor%20Object%20Reference))
  (bind _output_get (Variables|Default|SetActorAttached Target))
  (Transformation|AttachComponentToComponent _output_get (Variables|Default|GetTopOfCase) "None" "SnapToTarget" "KeepRelative" "KeepRelative" true)
  (Variables|Default|Setb_HaveSomethingOn true))

(fn OnDetached
  (bind _actorattached (Variables|Default|GetActorAttached))
  (Variables|Default|Setb_HaveSomethingOn false)
  (Utilities|IsValid _actorattached
    (:Is%20Valid
      (Transformation|DetachFromActor _actorattached "KeepRelative" "KeepRelative" "KeepRelative"))))