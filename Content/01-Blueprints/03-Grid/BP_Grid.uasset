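; BP_Grid is the game grid actor that spawns enemies on a designated set of its cases.
; On BeginPlay it casts eight specific child-actor cases to BP_Case and stores them as spawn candidates.
; SpawnEnemy picks a random unoccupied candidate, spawns the given BP_ParentEnemy class at its top transform and attaches the enemy to that case.
; If every candidate is occupied, nothing spawns.
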(event EventBeginPlay
  (CallFunction|GetSpawnableCase (Variables|Default|GetBP_Case25))
  (CallFunction|GetSpawnableCase (Variables|Default|GetBP_Case28))
  (CallFunction|GetSpawnableCase (Variables|Default|GetBP_Case16))
  (CallFunction|GetSpawnableCase (Variables|Default|GetBP_Case26))
  (CallFunction|GetSpawnableCase (Variables|Default|GetBP_Case31))
  (CallFunction|GetSpawnableCase (Variables|Default|GetBP_Case30))
  (CallFunction|GetSpawnableCase (Variables|Default|GetBP_Case27))
  (CallFunction|GetSpawnableCase (Variables|Default|GetBP_Case29)))

(fn ConstructionScript)

(fn SpawnEnemy
  (params (Class :type Actor%20Class%20Reference))
  (bind _temparrayofspawn (LocalVariables|GetTempArrayOfSpawn))
  (bind _asbp_parent_enemy (Utilities|Casting|CastToBP_ParentEnemyClass Class))
  (for _array_element (Variables|Default|GetCaseToSpawnArray)
    (if (not (Variables|/Game/01-Blueprints/03-Grid/BP_Case.BP_Case_C|Getb_HaveSomethingOn _array_element))
      (Utilities|Array|Add (LocalVariables|GetTempArrayOfSpawn) _array_element)))
  (if (Utilities|Array|IsEmpty _temparrayofspawn)
    (return)
    (else
      (bind _output_get (LocalVariables|SetCaseTemp (.OutItem (Utilities|Array|Random _temparrayofspawn))))
      (bind _returnvalue (Game|SpawnActorfromClass _asbp_parent_enemy (Transformation|GetWorldTransform (Variables|/Game/01-Blueprints/03-Grid/BP_Case.BP_Case_C|GetTopOfCase _output_get)) "AlwaysSpawn" "MultiplyWithRoot" 0 (LocalVariables|GetCaseTemp) 0))
      (Default|OnAttached (LocalVariables|GetCaseTemp) _returnvalue)
      (return))))

(fn GetSpawnableCase
  (params (BPCase :type Child%20Actor%20Component%20Object%20Reference))
  (bind _asbp_case (Utilities|Casting|CastToBP_Case (Variables|/Script/Engine.ChildActorComponent|GetChildActor BPCase)))
  (Utilities|Array|Add (Variables|Default|GetCaseToSpawnArray) _asbp_case))