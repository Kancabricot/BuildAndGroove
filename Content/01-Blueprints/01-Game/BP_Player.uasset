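; BP_Player is the player controller for card combat, handling the mouse cursor, card drag state and mana.
; BeginPlay adds the Enhanced Input mapping context, shows the cursor and fills mana to its maximum.
; OnDragCard stores the dragged card and line widget; releasing the left mouse button removes the widget and passes current mana to the card's drag-cancelled event.
; Mana changes are pushed to the combat HUD through the GameMode.
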(event Custom|OnDragCard
  (params (WG_DrawLineRef :type WG%20Draw%20Line%20Object%20Reference) (ActualCard :type WG%20Card%20Object%20Reference))
  (Variables|Default|SetWG_DrawLineRef WG_DrawLineRef)
  (Variables|Default|SetActualCard ActualCard)
  (Variables|Default|Setb_InDrag true))

(event EventBeginPlay
  (Variables|Default|SetGame%20Mode (CallFunction|GetGameMode self))
  (Input|AddMappingContext (PlayerController|LocalPlayerSubsystems|GetEnhancedInputLocalPlayerSubsystem self) "/Game/10-Inputs/IMC_Player.IMC_Player" 0 "(bIgnoreAllPressedKeysUntilRelease=True,bForceImmediately=False,bNotifyUserSettings=False)")
  (Variables|Default|SetbShowMouseCursor true)
  (CallFunction|SetManatoManaMax))

(event Input|MouseEvents|LeftMouseButton
  (params (Key :type Key%20Structure :default "None"))
  (:Released
    (if (Variables|Default|Getb_InDrag)
      (Variables|Default|Setb_InDrag false)
      (Widget|RemovefromParent (Variables|Default|GetWG_DrawLineRef))
      (Default|EventonDragCancelled (Variables|Default|GetActualCard) (Variables|Default|GetActualMana)))))

(fn ConstructionScript)

(fn ChangeManaValue
  (params (B :type Integer))
  (bind _output_get (Variables|Default|SetActualMana (+ (Variables|Default|GetActualMana) B)))
  (Default|ManaInfo (Variables|/Game/01-Blueprints/01-Game/BP_GameModeCombat.BP_GameModeCombat_C|GetHUDCombat (Variables|Default|GetGame%20Mode)) _output_get (Variables|Default|GetManaMax)))

(fn SetManatoManaMax
  (bind _output_get (Variables|Default|SetActualMana (Variables|Default|GetManaMax)))
  (Default|ManaInfo (Variables|/Game/01-Blueprints/01-Game/BP_GameModeCombat.BP_GameModeCombat_C|GetHUDCombat (Variables|Default|GetGame%20Mode)) _output_get (Variables|Default|GetManaMax)))