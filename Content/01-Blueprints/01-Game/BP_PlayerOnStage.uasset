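; Player actor on the stage of what appears to be a card game, holding life and shield and driving a life bar widget.
; BeginPlay caches the widget component's WG_LifeBar and resets life to maximum.
; TakeDamage lets the shield absorb hits first, passes overflow to life, updates the bar and opens the lose menu at zero.
; GetShield raises the shield display, while card hover events forward to its BPCase.
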(event EventBeginPlay
  (bind _aswg_life_bar (Utilities|Casting|CastToWG_LifeBar (UserInterface|GetWidget (Variables|Default|GetWG_LifeBar))))
  (Variables|Default|SetLifeBarRef _aswg_life_bar)
  (CallFunction|ResetLife)
  (Default|OnBarChange (Variables|Default|GetLifeBarRef) (Variables|Default|GetPlayerLife) (Variables|Default|GetPlayerMaxLife)))

(fn ConstructionScript)

(fn OnCardHover
  (Utilities|IsValid (Variables|Default|GetBP_Case)
    (:Is%20Valid
      (Default|OnHover (Variables|Default|GetBP_Case)))))

(fn OnCardUnhover
  (Utilities|IsValid (Variables|Default|GetBP_Case)
    (:Is%20Valid
      (Default|OnUnhover (Variables|Default|GetBP_Case)))))

(fn TakeDamage
  (params (Damage :type Integer))
  (bind (_needdamage _damage) (CallFunction|CheckShield Damage))
  (if _needdamage
    (bind _output_get (Variables|Default|SetPlayerLife (- (Variables|Default|GetPlayerLife) _damage)))
    (Default|OnBarChange (Variables|Default|GetLifeBarRef) _output_get (Variables|Default|GetPlayerMaxLife))
    (if (<= _output_get 0)
      (CallFunction|Loose))))

(fn ResetLife
  (Variables|Default|SetPlayerLife (Variables|Default|GetPlayerMaxLife)))

(fn Loose
  (bind _returnvalue (UserInterface|CreateWidget "/Game/03-Widgets/WG_MenuLoose.WG_MenuLoose_C"))
  (UserInterface|Viewport|AddtoViewport _returnvalue 0))

(fn GetShield
  (params (Shield :type Integer))
  (if (> (Variables|Default|GetShield) 0)
    _
    (else
      (Default|ShowMaskShield (Variables|Default|GetLifeBarRef) true)))
  (bind _output_get (Variables|Default|SetShield (+ (Variables|Default|GetShield) Shield)))
  (Default|OnChangeShield (Variables|Default|GetLifeBarRef) _output_get))

(fn CheckShield
  (params (DamageTake :type Integer))
  (if (> (Variables|Default|GetShield) 0)
    (LocalVariables|SetDamageTaken (- (Variables|Default|GetShield) DamageTake))
    (if (< (- (Variables|Default|GetShield) DamageTake) 0)
      (Variables|Default|SetShield 0)
      (Default|ShowMaskShield (Variables|Default|GetLifeBarRef) false)
      (return true (Math|Integer|Absolute(Integer) (LocalVariables|GetDamageTaken)))
      (else
        (bind _output_get (Variables|Default|SetShield (LocalVariables|GetDamageTaken)))
        (Default|OnChangeShield (Variables|Default|GetLifeBarRef) _output_get)
        (return false 0)))
    (else
      (return true DamageTake))))