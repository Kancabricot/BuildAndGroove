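; Game mode for a grid-based card combat game that runs the turn loop as a chain of phase functions, each updating a combat state enum.
; BeginPlay creates the combat HUD, then after a short delay spawns the grid, points the camera at it and draws into the hand widget.
; The chain halts at the empty player main phase; StopMainPhasePlayer resumes it, discarding the hand and running placeholder enemy phases back into Draw.
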(event Custom|SpawnEnemyDebug
  (Default|SpawnEnemy (Variables|Default|GetGrid) "/Game/01-Blueprints/02-Enemys/BP_Dummy.BP_Dummy_C"))

(event EventBeginPlay
  (Variables|Default|SetEnum_CombatState "NewEnumerator9")
  (bind _returnvalue (UserInterface|CreateWidget "/Game/03-Widgets/WG_InGameInterface.WG_InGameInterface_C" 0 self))
  (UserInterface|Viewport|AddtoPlayerScreen _returnvalue)
  (Variables|Default|SetHUDCombat _returnvalue)
  (Input|SetInputModeGameandUI (Game|GetPlayerController 0) _returnvalue "DoNotLock" false false)
  (Utilities|FlowControl|Delay 0.5)
  (Phase|SpawnPhase))

(fn ConstructionScript)

(fn SpawnPhase
  ;[1 1 1] Spawn
  (CallFunction|SpawnMap)
  (Variables|Default|SetEnum_CombatState "NewEnumerator1")
  (Phase|DrawPhase))

(fn DrawPhase
  (for _index (range 0 0)
    (Default|DrawCard (Variables|/Game/03-Widgets/WG_InGameInterface.WG_InGameInterface_C|GetWG_Hand (Variables|Default|GetHUDCombat)) (Variables|Default|GetPlayerDeck)))
  (Variables|Default|SetEnum_CombatState "NewEnumerator2")
  (Phase|IntentionPhase))

(fn IntentionPhase
  (Variables|Default|SetEnum_CombatState "NewEnumerator3")
  (Phase|BeginPhasePlayer))

(fn BeginPhasePlayer
  (Variables|Default|SetEnum_CombatState "NewEnumerator4")
  (Phase|StartMainPhasePlayer))

(fn StartMainPhasePlayer)

(fn StopMainPhasePlayer
  (Variables|Default|SetEnum_CombatState "NewEnumerator5")
  (Phase|EndPhasePlayer))

(fn EndPhasePlayer
  (Variables|Default|SetEnum_CombatState "NewEnumerator6")
  (Phase|DiscardPhase))

(fn DiscardPhase
  (bind _hudcombat (Variables|Default|GetHUDCombat))
  (bind _wg_hand (Variables|/Game/03-Widgets/WG_InGameInterface.WG_InGameInterface_C|GetWG_Hand _hudcombat))
  (bind _cardinhand (Variables|/Game/03-Widgets/WG_Hand.WG_Hand_C|GetCardInHand _wg_hand))
  (if (Utilities|Array|IsEmpty _cardinhand)
    (Phase|BeginPhaseEnemy)
    (else
      (for _array_element _cardinhand
        (Default|DiscardCard _array_element)
        (Widget|RemovefromParent _array_element))
      (Utilities|Array|Clear _cardinhand)
      (Phase|BeginPhaseEnemy))))

(fn BeginPhaseEnemy
  (Variables|Default|SetEnum_CombatState "NewEnumerator7")
  (Phase|MainPhaseEnemy))

(fn MainPhaseEnemy
  (Variables|Default|SetEnum_CombatState "NewEnumerator8")
  (Phase|EndPhaseEnemy))

(fn EndPhaseEnemy
  (Variables|Default|SetEnum_CombatState "NewEnumerator3")
  (Phase|DrawPhase))

(fn SpawnMap
  (bind _returnvalue (Game|SpawnActorfromClass "/Game/01-Blueprints/03-Grid/BP_Grid.BP_Grid_C" (Math|Transform|MakeTransform "0, 0, 0" "0, 0, 0" "1.000000,1.000000,1.000000") "Undefined" "MultiplyWithRoot" 0 0))
  (bind _output_get (Variables|Default|SetGrid _returnvalue))
  (Game|Player|SetViewTargetwithBlend (Game|GetPlayerController 0) _output_get 0.0 "VTBlend_Linear" 0.0 false))

(fn Draw
  (Default|DrawCard (Variables|/Game/03-Widgets/WG_InGameInterface.WG_InGameInterface_C|GetWG_Hand (Variables|Default|GetHUDCombat)) (Variables|Default|GetPlayerDeck)))